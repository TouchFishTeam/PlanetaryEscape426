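; UITester is a trigger-box actor for previewing a UI material on screen while the player stands inside it.
; Player overlap creates a WidgetTester widget and passes it the test material, or a dynamic instance if enabled; leaving removes all widgets.
; With the dynamic option on, Tick animates the NoiseScale vector while any actor overlaps, oscillating G around its initial value and setting B to game time.
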(event OnComponentBeginOverlap(Box)
  (params (OverlappedComponent :type Primitive%20Component%20Object%20Reference) (OtherActor :type Actor%20Object%20Reference) (OtherComp :type Primitive%20Component%20Object%20Reference) (OtherBodyIndex :type Integer) (bFromSweep :type Boolean) (SweepResult :type Hit%20Result%20Structure%20%28by%20ref%29))
  (if (== OtherActor (Game|Player|GetPlayerPawn 0))
    (bind _returnvalue (UserInterface|CreateWidget (Variables|Default|GetWidgetTesterClass) (Game|GetPlayerController 0)))
    (UserInterface|Viewport|AddtoPlayerScreen _returnvalue)
    (bind _aswidget_tester (Utilities|Casting|CastToWidgetTester _returnvalue))
    (Default|SetMaterial _aswidget_tester (select (Variables|Default|GetCreateDynamicMaterial?) (Variables|Default|GetDMI) (Variables|Default|GetMaterialToTest)))))

(event OnComponentEndOverlap(Box)
  (params (OverlappedComponent :type Primitive%20Component%20Object%20Reference) (OtherActor :type Actor%20Object%20Reference) (OtherComp :type Primitive%20Component%20Object%20Reference) (OtherBodyIndex :type Integer))
  (if (== OtherActor (Game|Player|GetPlayerPawn 0))
    (Viewport|RemoveAllWidgets)))

(event EventBeginPlay
  (if (Variables|Default|GetCreateDynamicMaterial?)
    (bind _returnvalue (Rendering|Material|CreateDynamicMaterialInstance (Variables|Default|GetMaterialToTest) :!class /Script/Engine.KismetMaterialLibrary))
    (bind _output_get (Variables|Default|SetDMI _returnvalue))
    (bind _returnvalue_2 (Rendering|Material|GetVectorParameterValue _output_get "NoiseScale" :!class /Script/Engine.MaterialInstanceDynamic))
    (Variables|Default|SetNoiseScale _returnvalue_2)))

(event Collision|EventActorBeginOverlap
  (params (OtherActor :type Actor%20Object%20Reference)))

(event EventTick
  (params (DeltaSeconds :type Float%20%28single-precision%29))
  (bind _returnvalue (Utilities|Time|GetGameTimeinSeconds))
  (bind _noisescale (Variables|Default|GetNoiseScale))
  (if (and (Variables|Default|GetCreateDynamicMaterial?) (Math|Conversions|ToBoolean(Integer) (Utilities|Array|Length (Collision|GetOverlappingActors (Variables|Default|GetBox) 0 :!class /Script/Engine.PrimitiveComponent))))
    (Rendering|Material|SetVectorParameterValue (Variables|Default|GetDMI) "NoiseScale" (Math|Color|MakeColor (.r _noisescale) (+ (.g _noisescale) (* (Math|Trig|Sin(Radians) _returnvalue) 0.4)) _returnvalue (.a _noisescale)) :!class /Script/Engine.MaterialInstanceDynamic)))

(fn ConstructionScript)