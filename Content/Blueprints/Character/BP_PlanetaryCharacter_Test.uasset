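; Test player character that walks on planets under their gravity and flies by jetpack in space.
; Planet notifies maintain SavedPlanets; Tick sums their gravity as capsule forces, adds friction and aligns the body to traced surface normals.
; Input drives force-based walking, velocity-based double jumps, then a fuel-limited, camera-relative jetpack; off-planet, rotation lerps toward control rotation.
; Nozzle effects and velocity fading are unfinished or disconnected; several planet classes return no gravity scale.
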(event EventHitonLand
  (params (LastHitPlanet :type Actor%20Object%20Reference))
  ;[1 1 1] PlanetNotify
  ;;[1 1 1] GetIsOnLand And ResetJumpCount
  (Utilities|FlowControl|Sequence
    (:then_0
      (Variables|Default|SetIsOnLand true))
    (:then_1
      (Variables|Default|SetJumpCount 0))
    (:then_2
      (Variables|Default|SetEnableJetpackBySpaceKey false))
    (:then_3
      (Variables|Default|SetLastHitPlanet LastHitPlanet))))

(event EventLeaveCurrentPlanet
  (params (SavedPlanet :type Actor%20Object%20Reference))
  ;[1 1 1] PlanetNotify
  ;;[1 1 1] SetCurrentPlanet
  (Utilities|IsValid SavedPlanet
    (:Is%20Valid
      (Utilities|Array|RemoveItem (Variables|Default|GetSavedPlanets) SavedPlanet)
      ;;;[1 1 1] Set IsOnPlanet False Only When SavedPlanets Is Empty
      (if (== (Utilities|Array|Length (Variables|Default|GetSavedPlanets)) 0)
        (Variables|Default|SetIsOnPlanet false)))))

(event EventTick
  (params (DeltaSeconds :type Float%20%28single-precision%29))
  ;[1 1 1] AdjustMovement
  (if (Variables|Default|GetIsOnPlanet)
    ;;[1 1 1] AdujstMovement Only When OnPlanet
    (Utilities|FlowControl|Sequence
      (:then_0
        ;;;[1 1 1] AdjustRotation
        ;;;;[1 1 1] Press"R"ToResetRotation
        (if (not (Variables|Default|GetIsResetingRotation))
          ;;;;[1 1 1] IfLastHirPlanetExist
          (Utilities|IsValid (Variables|Default|GetLastHitPlanet)
            (:Is%20Valid
              ;;;;[1 1 1] GetSurfaceNormal(HaveChanceToHitOnOtherThing)
              (bind _outhit (Collision|SphereTraceByChannel (Transformation|GetWorldLocation (Variables|Character|GetMesh)) (Transformation|GetActorLocation (Variables|Default|GetLastHitPlanet)) 2.0 "TraceTypeQuery1" false 0 "None"))
              (Variables|Default|SetTmpNormalVector (.ImpactNormal (Collision|BreakHitResult _outhit)))
              (if (!= (Utilities|Array|FindItem (Variables|Default|GetSavedPlanets) (.HitActor (Collision|BreakHitResult _outhit))) -1)
                ;;;;[1 1 1] CalcuateAndApplyRotation
                (bind _alpha (Timeline|EaseRotTimeline Play)
                  (:Update
                    (if (Variables|Default|GetIsOnPlanet)
                      (Transformation|SetActorRotation (Math|Interpolation|Ease "Linear" _alpha (Pawn|GetControlRotation :!class /Script/Engine.Pawn) (Math|Rotator|MakeRotfromZX (Variables|Default|GetTmpNormalVector) (Math|Vector|GetForwardVector (Pawn|GetControlRotation :!class /Script/Engine.Pawn))) true))))))))
          (else
            ;;;;[1 1 1] GetPlanerPointToPlayerNormal
            (Variables|Default|SetTmpNormalVector (Math|Vector|GetForwardVector (Math|Rotator|FindLookatRotation (Transformation|GetActorLocation (Variables|Default|GetLastHitPlanet)) (Transformation|GetActorLocation))))
            (Timeline|EaseRotTimeline PlayFromStart))))
      (:then_1
        ;;;[1 1 1] Gravity
        ;;;;[1 1 1] CalcuateGravityVector
        (Variables|Default|SetTmpGravityVector "0, 0, 0")
        (for _array_element (Variables|Default|GetSavedPlanets)
          (bind _gravityscale (CallFunction|GetPlanetGravityScale _array_element))
          (Variables|Default|SetTmpGravityVector (+ (Variables|Default|GetTmpGravityVector) (* (Math|Vector|GetForwardVector (Math|Rotator|FindLookatRotation (Transformation|GetActorLocation _array_element) (Transformation|GetActorLocation))) _gravityscale))))
        ;;;;[1 1 1] ApplyGravity
        (Physics|AddForce (Variables|Collision|GetCapsuleComponent) (* (* (Variables|Default|GetTmpGravityVector) -1.0) (Variables|Default|GetPhysGravityForce)) "None" false))
      (:then_2
        ;;;[1 1 1] Friction (Only When IsOnLand)
        (if (Variables|Default|GetIsOnLand)
          (Physics|AddForce (Variables|Collision|GetCapsuleComponent) (* (Math|Vector|Normalize (Transformation|GetVelocity (Game|Player|GetPlayerPawn 0))) (* (Variables|Default|GetPhysFrictionForce) -1.0)) "None" false)))
      (:then_3
        ;;;[1 1 1] RecoverJetpackTimeWhenNoJumpInput
        (bind _yes (CallFunction|IsMoveInputorNot))
        (if (not _yes)
          (if (< (Variables|Default|GetTime) (Variables|Default|GetMaxTime))
            (Utilities|FlowControl|Delay 1.0)
            (Variables|Default|SetTime (+ (Variables|Default|GetTime) 1))))))
    (else
      ;;[1 1 1] AdujstMovement Only When OnOuterSpace
      ;;;[1 1 1] AdjustRotation LinearLerp
      (Utilities|FlowControl|Sequence
        (:then_0
          (Transformation|SetActorRotation (Math|Rotator|Lerp(Rotator) (Transformation|GetActorRotation) (Pawn|GetControlRotation :!class /Script/Engine.Pawn) 0.01 true)))))))

(event EventBeginPlay
  ;[1 1 1] Init
  ;;[1 1 1] Get Jetpack
  (Transformation|AttachComponentToComponent (Variables|Default|GetJetpack) (Variables|Character|GetMesh) "JetpackSocket" "SnapToTarget" "SnapToTarget" "KeepWorld" true)
  (Variables|Default|SetIsOnLand true))

(event EventApproachNewPlanet
  (params (NewPlanet :type Actor%20Object%20Reference))
  ;[1 1 1] PlanetNotify
  ;;[1 1 1] SetCurrentPlanet
  (Utilities|IsValid NewPlanet
    (:Is%20Valid
      (Utilities|Array|Insert (Variables|Default|GetSavedPlanets) NewPlanet)
      (Variables|Default|SetIsOnPlanet true)
      (Components|Timeline|PlayfromStart (Variables|Default|GetEaseRotTimeline)))))

(event Input|ActionEvents|InputActionEscape
  (params (Key :type Key%20Structure))
  (bind _returnvalue (Game|GetPlayerController 0))
  ;[1 1 1] Esc HUD
  (:Pressed
    (bind _returnvalue_2 (UserInterface|CreateWidget "/Game/UMG/Ingame_esc.Ingame_esc_C" _returnvalue))
    (Input|SetInputModeUIOnly _returnvalue 0 "DoNotLock")
    (Game|SetGamePaused true)
    (Variables|/Script/Engine.PlayerController|SetbShowMouseCursor _returnvalue true)
    (UserInterface|Viewport|AddtoViewport _returnvalue_2 0)))

(event Input|ActionEvents|InputActionResetRotation
  (params (Key :type Key%20Structure))
  ;[1 1 1] ResetRotation
  (:Pressed
    (Variables|Default|SetIsResetingRotation true))
  (:Released
    (Variables|Default|SetIsResetingRotation false)))

(event Input|AxisEvents|InputAxisJump
  (params (AxisValue :type Float%20%28single-precision%29))
  ;[1 1 1] Movement: MoveAndJump
  ;;[1 1 1] IsJumpKeyPressed
  (Variables|Default|SetCurrJumpAxisValue AxisValue)
  ;;[1 1 1] JumpOrJetpackOrNot
  ;;;[1 1 1] ShouldUseJetpack If InOuterSpace And HaveMoveInput
  (bind _yes (CallFunction|IsMoveInputorNot))
  (if (and (or _yes (!= (Variables|Default|GetCurrJumpAxisValue) 0.0)) (not (Variables|Default|GetIsOnPlanet)))
    (CallFunction|JetpackFire :!label _label)
    (else
      ;;;[1 1 1] ShouldUseJetpack If IsOnPlanet And JumpCount>1
      (if (> (Variables|Default|GetJumpCount) 1)
        ;;;[1 1 1] Even Though ShouldUseJetpack If IsOnPlanet And JumpCount>1 But Should WaitForUseDelay After JumpTwice
        (if (Variables|Default|GetEnableJetpackBySpaceKey)
          (goto _label))
        (else
          (CallFunction|JumponPlanet))))))

(event Input|AxisEvents|InputAxisLookUp
  (params (AxisValue :type Float%20%28single-precision%29))
  ;[1 1 1] CameraRotate
  (Pawn|Input|AddControllerPitchInput (* (Variables|Default|GetMouseSensi) AxisValue)))

(event Input|AxisEvents|InputAxisTurn
  (params (AxisValue :type Float%20%28single-precision%29))
  ;[1 1 1] CameraRotate
  (Pawn|Input|AddControllerYawInput (* AxisValue (Variables|Default|GetMouseSensi))))

(event Input|AxisEvents|InputAxisMoveForward
  (params (AxisValue :type Float%20%28single-precision%29))
  ;[1 1 1] Movement: MoveAndJump
  ;;[1 1 1] IsMoveKeyPressed
  (Variables|Default|SetCurrMoveForwardAxisValue AxisValue)
  ;;[1 1 1] Move Input Handler
  (Utilities|FlowControl|Sequence
    (:then_0
      ;;;[1 1 1] ShouldUseJetpackToMoveOrNot
      (bind _use (CallFunction|ShouldUseJetpacktoMoveorNot))
      (if _use
        (bind _yes (CallFunction|IsMoveInputorNot))
        (if _yes
          (CallFunction|JetpackFire)
          (else
            (Variables|Default|SetNozzleFirePushDirection "0, 0, 0")))
        (else
          (CallFunction|MoveonPlanet))))
    (:then_1
      ;;;[1 1 1] Set LastInputAxisValueInTheEnd
      (Variables|Default|SetLastMoveForwardAxisValue (Variables|Default|GetCurrMoveForwardAxisValue))
      (Variables|Default|SetLastMoveRightAxisValue (Variables|Default|GetCurrMoveRightAxisValue)))))

(event Input|AxisEvents|InputAxisMoveRight
  (params (AxisValue :type Float%20%28single-precision%29))
  ;[1 1 1] Movement: MoveAndJump
  ;;[1 1 1] IsMoveKeyPressed
  (Variables|Default|SetCurrMoveRightAxisValue AxisValue)
  ;;[1 1 1] Move Input Handler
  (Utilities|FlowControl|Sequence
    (:then_0
      ;;;[1 1 1] ShouldUseJetpackToMoveOrNot
      (bind _use (CallFunction|ShouldUseJetpacktoMoveorNot))
      (if _use
        (bind _yes (CallFunction|IsMoveInputorNot))
        (if _yes
          (CallFunction|JetpackFire)
          (else
            (Variables|Default|SetNozzleFirePushDirection "0, 0, 0")))
        (else
          (CallFunction|MoveonPlanet))))
    (:then_1
      ;;;[1 1 1] Set LastInputAxisValueInTheEnd
      (Variables|Default|SetLastMoveForwardAxisValue (Variables|Default|GetCurrMoveForwardAxisValue))
      (Variables|Default|SetLastMoveRightAxisValue (Variables|Default|GetCurrMoveRightAxisValue)))))

(fn ConstructionScript)

(fn GetPlanetGravityScale
  (params (Planet :type Actor%20Object%20Reference))
  (bind _asbp_planet (Utilities|Casting|CastToBP_Planet Planet)
    (:then
      (return (Variables|/Game/Blueprints/Mesh/BP_Planet.BP_Planet_C|GetGravityScale _asbp_planet)))
    (:CastFailed
      (bind _asbp_planet_3 (Utilities|Casting|CastToBP_Planet3 Planet)
        (:then
          (return (Variables|/Game/Blueprints/Mesh/BP_Planet3.BP_Planet3_C|GetGravityScale _asbp_planet_3)))
        (:CastFailed
          (bind _asbp_ship (Utilities|Casting|CastToBP_Ship Planet)
            (:CastFailed
              (bind _asbp_planet_1 (Utilities|Casting|CastToBP_Planet_1 Planet)
                (:CastFailed
                  (bind _asbp_planet_2 (Utilities|Casting|CastToBP_Planet_2 Planet)
                    (:CastFailed
                      (bind _asbp_planet_3_2 (Utilities|Casting|CastToBP_Planet_3 Planet)
                        (:then
                          (return (Variables|/Game/Blueprints/Mesh/BP_Planet_3.BP_Planet_3_C|GetGarvityScale _asbp_planet_3_2)))
                        (:CastFailed
                          (bind _asbp_rock_1 (Utilities|Casting|CastToBP_Rock_1 Planet)
                            (:then
                              (return (Variables|/Game/Blueprints/Mesh/BP_Rock_1.BP_Rock_1_C|GetGarvityScale _asbp_rock_1)))
                            (:CastFailed
                              (bind _asbp_rock_2 (Utilities|Casting|CastToBP_Rock_2 Planet)
                                (:then
                                  (return (Variables|/Game/Blueprints/Mesh/BP_Rock_2.BP_Rock_2_C|GetGarvityScale _asbp_rock_2)))
                                (:CastFailed
                                  (bind _asbp_rock_3 (Utilities|Casting|CastToBP_Rock_3 Planet)
                                    (:CastFailed
                                      (bind _asbp_rock_field (Utilities|Casting|CastToBP_RockField Planet)
                                        (:then
                                          (return (Variables|/Game/Blueprints/Mesh/BP_RockField.BP_RockField_C|GetGarvityScale _asbp_rock_field)))
                                        (:CastFailed
                                          (bind _asbp_round_rock_1 (Utilities|Casting|CastToBP_RoundRock_1 Planet)
                                            (:then
                                              (return (Variables|/Game/Blueprints/Mesh/BP_RoundRock_1.BP_RoundRock_1_C|GetGarvityScale _asbp_round_rock_1)))
                                            (:CastFailed
                                              (bind _asbp_round_rock_2 (Utilities|Casting|CastToBP_RoundRock_2 Planet))
                                              (return (Variables|/Game/Blueprints/Mesh/BP_RoundRock_2.BP_RoundRock_2_C|GetGarvityScale _asbp_round_rock_2)))))))))))))))))))))))))

(fn IsMoveInputorNot
  ;[1 1 1] If IsMoving
  (if (not (and (== (Variables|Default|GetCurrMoveRightAxisValue) 0.0) (== (Variables|Default|GetCurrMoveForwardAxisValue) 0.0)))
    (return true)
    (else
      (return false))))

(fn ShouldUseJetpacktoMoveorNot
  (if (or (> (Variables|Default|GetJumpCount) 2) (not (Variables|Default|GetIsOnPlanet)))
    (return true)
    (else
      (return false))))

(fn IfMoveDirChange
  (if (or (!= (Variables|Default|GetCurrMoveRightAxisValue) (Variables|Default|GetLastMoveRightAxisValue)) (!= (Variables|Default|GetCurrMoveForwardAxisValue) (Variables|Default|GetLastMoveForwardAxisValue)))
    (return true)
    (else
      (return false))))

(fn IsonPlanetorNot
  ;[1 1 1] If OnPlanet
  (if (Variables|Default|GetIsOnPlanet)
    (return true)
    (else
      (return false))))

(fn GetCurrMoveDir
  (Variables|Default|SetTmpDirVector "0, 0, 0")
  (Utilities|FlowControl|Sequence
    (:then_0
      (Variables|Default|SetTmpDirVector (+ (Variables|Default|GetTmpDirVector) (* (Math|Vector|GetForwardVector (Variables|Collision|GetCapsuleComponent)) (Variables|Default|GetCurrMoveForwardAxisValue)))))
    (:then_1
      (Variables|Default|SetTmpDirVector (+ (Variables|Default|GetTmpDirVector) (* (Math|Vector|GetForwardVector (Variables|Collision|GetCapsuleComponent)) (Variables|Default|GetCurrMoveRightAxisValue)))))
    (:then_2
      (return (Variables|Default|GetTmpDirVector)))))

(fn IsJmpingorNot
  (if (Variables|Default|GetIsJumpAnimPlaying)
    (return true)))

(fn JetpackFire
  (bind _currentnozzles (Variables|Default|GetCurrentNozzles))
  ;[1 1 1] If NozzlesShouldChange
  (bind _hadchange (CallFunction|IfMoveDirChange))
  (if (or (or _hadchange (!= (Variables|Default|GetLastJumpAxisValue) (Variables|Default|GetCurrJumpAxisValue))) (Math|Vector|Equal(Vector) (Variables|Default|GetNozzleFirePushDirection) "0, 0, 0" 0.0001))
    (Utilities|FlowControl|Sequence
      (:then_0
        ;[1 1 1] SetNewNozzles
        (Utilities|Array|Clear (Variables|Default|GetCurrentNozzles)))
      (:then_1
        ;;[1 1 1] ShouldUseJetpackToMove: SelectNozzles
        (if (== (Variables|Default|GetCurrMoveRightAxisValue) 1.0)
          (Utilities|Array|Insert _currentnozzles (Variables|Default|GetLeftNozzle1))
          (Utilities|Array|Insert _currentnozzles 0)))
      (:then_2
        (if (== (Variables|Default|GetCurrMoveRightAxisValue) -1.0)
          _))
      (:then_3
        (if (== (Variables|Default|GetCurrMoveForwardAxisValue) 1.0)
          _))
      (:then_4
        ;;[1 1 1] ShouldUseJetpackToJump: SelectNozzles
        (if (== (Variables|Default|GetCurrJumpAxisValue) 1.0)
          _))
      (:then_5
        ;[1 1 1] SetNozzleFirePushDirection
        (Variables|Default|SetNozzleFirePushDirection "0, 0, 0"))
      (:then_6
        (Variables|Default|SetNozzleFirePushDirection (+ (* (Math|Vector|GetRightVector (Variables|MyCharacter|GetFollowCamera)) (Variables|Default|GetCurrMoveRightAxisValue)) (Variables|Default|GetNozzleFirePushDirection))))
      (:then_7
        (Variables|Default|SetNozzleFirePushDirection (+ (* (Math|Vector|GetForwardVector (Variables|MyCharacter|GetFollowCamera)) (Variables|Default|GetCurrMoveForwardAxisValue)) (Variables|Default|GetNozzleFirePushDirection))))
      (:then_8
        (Variables|Default|SetNozzleFirePushDirection (+ (* (Math|Vector|GetUpVector (Variables|MyCharacter|GetFollowCamera)) (Variables|Default|GetCurrJumpAxisValue)) (Variables|Default|GetNozzleFirePushDirection))))
      (:then_9
        ;[1 1 1] IfJetpackTimeRemaining
        (if (> (Variables|Default|GetTime) 0) :!label _label
          ;[1 1 1] UseJetpack
          (Utilities|FlowControl|Sequence
            (:then_0
              ;;[1 1 1] ApplyFireEffectForEachJetpackNozzles
              (for _array_element (Variables|Default|GetCurrentNozzles)
                (bind _asarrow_component (Utilities|Casting|CastToArrowComponent _array_element))))
            (:then_1
              ;;[1 1 1] ApplyJetpackForce
              (Physics|AddForce (Variables|Collision|GetCapsuleComponent) (* (Variables|Default|GetNozzleFirePushDirection) (Variables|Default|GetPhysJetpackForce)) "None" false))
            (:then_2
              ;;[1 1 1] ReduceJetpackTime
              (Variables|Default|SetFloatToIntTimer (- (Variables|Default|GetFloatToIntTimer) 0.1))
              (if (< (Variables|Default|GetFloatToIntTimer) 0.0)
                (Variables|Default|SetFloatToIntTimer 4.0)
                (Variables|Default|SetTime (- (Variables|Default|GetTime) 1))))))))
    (else
      (goto _label))))

(fn MoveonPlanet
  (bind _capsulecomponent (Variables|Collision|GetCapsuleComponent))
  (bind _capsulecomponent_2 (Variables|Collision|GetCapsuleComponent))
  ;[1 1 1] OnlyOnPlanet
  (bind _yes (CallFunction|IsonPlanetorNot))
  (if _yes
    (Utilities|FlowControl|Sequence
      (:then_0
        ;[1 1 1] IfPhysLinearVelcoityCanIncrease
        (bind _returnvalue (Physics|GetPhysicsLinearVelocity (Variables|Collision|GetCapsuleComponent) "None"))
        (if (<= (Math|Vector|VectorLength _returnvalue) (Variables|Default|GetPhysWalkMaxSpeed))
          ;[1 1 1] PhysLinearVelcoityIncrease ByAddForce
          (Utilities|FlowControl|Sequence
            (:then_0
              (Physics|AddForce _capsulecomponent_2 (* (* (Math|Vector|GetRightVector _capsulecomponent_2) (Variables|Default|GetCurrMoveRightAxisValue)) (Variables|Default|GetPhysWalkAcceleration)) "None" false))
            (:then_1
              (Physics|AddForce _capsulecomponent (* (* (Math|Vector|GetForwardVector _capsulecomponent) (Variables|Default|GetCurrMoveForwardAxisValue)) (Variables|Default|GetPhysWalkAcceleration)) "None" false))))))))

(fn JumponPlanet
  (bind _capsulecomponent (Variables|Collision|GetCapsuleComponent))
  (bind _physjumpspeed (Variables|Default|GetPhysJumpSpeed))
  (bind _returnvalue (Math|Vector|GetUpVector _capsulecomponent))
  (bind _returnvalue_2 (* _returnvalue _physjumpspeed))
  ;[1 1 1] ShouldNotUseJetpackToJump: Jump OnlyOnPlanet And OnlyTwice After HitOnLand
  ;;[1 1 1] JumpGate For Avoiding SecondJumpStartImmediatelyAfterFirstJump
  (if (and (Variables|Default|GetPassJumpInterval) (== (Variables|Default|GetCurrJumpAxisValue) 1.0))
    ;;[1 1 1] JumpStart
    (Utilities|FlowControl|Sequence
      (:then_0
        (Variables|Default|SetIsOnLand false)
        (Variables|Default|SetPassJumpInterval false)
        (Variables|Default|SetIsJumpAnimPlaying true))
      (:then_1
        ;;;[1 1 1] AddJumpVelocity
        (Physics|SetPhysicsLinearVelocity (Variables|Collision|GetCapsuleComponent) _returnvalue_2 true "None")
        (Development|PrintString (Utilities|String|ToString(Vector) _returnvalue_2)))
      (:then_2
        ;;[1 1 1] AfterJumpStart
        (Utilities|FlowControl|Sequence
          (:then_0
            ;;;[1 1 1] JumpCount++
            (Variables|Default|SetJumpCount (+ (Variables|Default|GetJumpCount) 1)))
          (:then_1
            ;;;[1 1 1] JumpInputInterval
            (Variables|Default|SetPassJumpInterval true))
          (:then_2
            ;;;[1 1 1] IntervalAfterJumpTwiceForEnableJetpack
            (if (== (Variables|Default|GetJumpCount) 2)
              (Variables|Default|SetEnableJetpackBySpaceKey true))))))))