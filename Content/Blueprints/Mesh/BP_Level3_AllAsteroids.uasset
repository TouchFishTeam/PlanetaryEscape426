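; Level 3 asteroid group actor, set up to swing all of its static mesh components together.
; BeginPlay caches the meshes, and Tick calls Play on SwingTimeline every frame.
; Each timeline update adds an unswept, cumulative world offset, lerped per axis between positive and negative swing distances, so the Alpha track drives step size rather than position.
; On finish, the timeline calls Reverse, though Tick keeps requesting forward play.
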(event Custom|Reverse
  (bind _swingdistancey (Variables|Default|GetSwingDistanceY))
  (bind _swingdistancez (Variables|Default|GetSwingDistanceZ))
  (bind _swingdistancex (Variables|Default|GetSwingDistanceX))
  ;[1 1 1] Swing
  (bind _alpha (Timeline|SwingTimeline Reverse)
    (:Update
      (for _array_element (Variables|Default|GetAllComponents)
        (Transformation|AddWorldOffset _array_element (Math|Vector|MakeVector (Math|Float|Lerp _swingdistancex (* _swingdistancex -1.0) _alpha) (Math|Float|Lerp _swingdistancey (* _swingdistancey -1.0) _alpha) (Math|Float|Lerp _swingdistancez (* _swingdistancez -1.0) _alpha)) false false)))
    (:Finished
      (CallFunction|Reverse))))

(event EventBeginPlay
  ;[1 1 1] GetAllComponents
  (Variables|Default|SetAllComponents (Actor|GetComponentsByClass "/Script/Engine.StaticMeshComponent")))

(event EventTick
  (params (DeltaSeconds :type Float%20%28single-precision%29))
  (bind _swingdistancey (Variables|Default|GetSwingDistanceY))
  (bind _swingdistancez (Variables|Default|GetSwingDistanceZ))
  (bind _swingdistancex (Variables|Default|GetSwingDistanceX))
  ;[1 1 1] Swing
  (bind _alpha (Timeline|SwingTimeline Play)
    (:Update
      (for _array_element (Variables|Default|GetAllComponents)
        (Transformation|AddWorldOffset _array_element (Math|Vector|MakeVector (Math|Float|Lerp _swingdistancex (* _swingdistancex -1.0) _alpha) (Math|Float|Lerp _swingdistancey (* _swingdistancey -1.0) _alpha) (Math|Float|Lerp _swingdistancez (* _swingdistancez -1.0) _alpha)) false false)))
    (:Finished
      (CallFunction|Reverse))))

(fn ConstructionScript)