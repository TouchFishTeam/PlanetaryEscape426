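; BP_Planet_3 is a planet actor that tells the player character when it enters or leaves the planet's atmosphere or hits its surface.
; Begin and end overlaps on the PlanetAtmosphere component send approach and leave messages, and the actor's Hit event sends a land-hit message.
; Each event reacts only to player character 0 and passes the planet itself, leaving the response to the character.
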(event OnComponentBeginOverlap(PlanetAtmosphere)
  (params (OverlappedComponent :type Primitive%20Component%20Object%20Reference) (OtherActor :type Actor%20Object%20Reference) (OtherComp :type Primitive%20Component%20Object%20Reference) (OtherBodyIndex :type Integer) (bFromSweep :type Boolean) (SweepResult :type Hit%20Result%20Structure%20%28by%20ref%29))
  (bind _returnvalue (Game|GetPlayerCharacter 0))
  ;[1 1 1] NotifyNewPlanet
  (if (== OtherActor _returnvalue)
    (Class|BPIGetIsonPlanet|ApproachNewPlanet(Message) _returnvalue self)))

(event OnComponentEndOverlap(PlanetAtmosphere)
  (params (OverlappedComponent :type Primitive%20Component%20Object%20Reference) (OtherActor :type Actor%20Object%20Reference) (OtherComp :type Primitive%20Component%20Object%20Reference) (OtherBodyIndex :type Integer))
  (bind _returnvalue (Game|GetPlayerCharacter 0))
  ;[1 1 1] NotifyNewPlanet
  (if (== OtherActor _returnvalue)
    (Class|BPIGetIsonPlanet|LeaveCurrentPlanet(Message) _returnvalue self)))

(event Collision|EventHit
  (params (MyComp :type Primitive%20Component%20Object%20Reference) (Other :type Actor%20Object%20Reference) (OtherComp :type Primitive%20Component%20Object%20Reference) (bSelfMoved :type Boolean) (HitLocation :type Vector :default "0, 0, 0") (HitNormal :type Vector :default "0, 0, 0") (NormalImpulse :type Vector :default "0, 0, 0") (Hit :type Hit%20Result%20Structure%20%28by%20ref%29))
  (bind _returnvalue (Game|GetPlayerCharacter 0))
  ;[1 1 1] NotifyHitLand
  (if (== Other _returnvalue)
    (Class|BPIGetIsonPlanet|HitonLand(Message) _returnvalue self)))

(fn ConstructionScript)