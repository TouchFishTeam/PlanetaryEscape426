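; BP_Level2_AllAsteroids is an actor that animates the Level 2 asteroids as an orbiting field.
; On BeginPlay it caches all of its static mesh components.
; Each Tick rotates their relative locations around the planet-ring mesh's up vector and spins each around its own up axis by a small random angle.
; Both motions use per-frame steps without delta time, so speed follows frame rate.
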(event EventBeginPlay
  ;[1 1 1] GetAllComponents
  (Variables|Default|SetAllComonents (Actor|GetComponentsByClass "/Script/Engine.StaticMeshComponent")))

(event EventTick
  (params (DeltaSeconds :type Float%20%28single-precision%29))
  (for _array_element (Variables|Default|GetAllComonents)
    (Utilities|FlowControl|Sequence
      (:then_0
        ;[1 1 1] OrientRotation
        (Transformation|SetRelativeLocation _array_element (Math|Vector|RotateVectorAroundAxis (Variables|/Script/Engine.SceneComponent|GetRelativeLocation _array_element) 0.05 (Math|Vector|GetUpVector (Variables|Default|GetSM_Env_Planet_Rings_01_StaticMeshComponent0))) false false))
      (:then_1
        ;[1 1 1] SelfRotation
        (Transformation|AddWorldRotation _array_element (Math|Vector|RotatorfromAxisandAngle (Math|Vector|GetUpVector _array_element) (Math|Random|RandomFloatinRange 0.0 0.05)) false false)))))

(fn ConstructionScript)