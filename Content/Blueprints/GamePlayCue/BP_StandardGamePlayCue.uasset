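; BP_StandardGamePlayCue is a cue actor that plays a sound and a particle effect on the player character.
; BeginPlay spawns both attached to player 0's root component and stores the components.
; Tick polls IsToDestroy, then pauses and destroys both components, stops the stored camera shake and destroys the actor.
; The camera shake is never started, as that logic is disconnected.
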(event EventBeginPlay
  ;[1 1 1] GamePlay
  (Utilities|FlowControl|Sequence
    (:then_0
      (bind _returnvalue (Audio|SpawnSoundAttached (Variables|Default|GetSoundToPlay) (Variables|/Script/Engine.Actor|GetRootComponent (Game|GetPlayerCharacter 0)) "None" "0, 0, 0" "0, 0, 0" "KeepRelativeOffset" true 1.0 1.0 0.0 0 0 false))
      (Variables|Default|SetSoundComp _returnvalue))
    (:then_1
      (bind _returnvalue_2 (Niagara|SpawnSystemAttached (Variables|Default|GetEmitterTemplateToPlay) (Variables|/Script/Engine.Actor|GetRootComponent (Game|GetPlayerCharacter 0)) "None" "0, 0, 0" "0, 0, 0" "KeepRelativeOffset" false))
      (Variables|Default|SetEffectComp _returnvalue_2))
    (:then_2)))

(event EventTick
  (params (DeltaSeconds :type Float%20%28single-precision%29))
  (bind _soundcomp (Variables|Default|GetSoundComp))
  (bind _effectcomp (Variables|Default|GetEffectComp))
  ;[1 1 1] Destroy
  (if (Variables|Default|GetIsToDestroy)
    (Utilities|FlowControl|Sequence
      (:then_0
        (Utilities|IsValid _soundcomp
          (:Is%20Valid
            (Class|AudioComponent|SetPaused _soundcomp true)
            (Components|DestroyComponent _soundcomp))))
      (:then_1
        (Utilities|IsValid _effectcomp
          (:Is%20Valid
            (Class|NiagaraComponent|SetPaused _effectcomp true)
            (Components|DestroyComponent _effectcomp))))
      (:then_2
        (CameraShakes|StopCameraShake (Game|GetPlayerCameraManager 0) (Variables|Default|GetCameraShakeComp) true))
      (:then_3
        (Actor|DestroyActor)))))

(fn ConstructionScript)